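; Player controller for SpeedBall that turns player input into physics-driven rolling and jumping of a ball.
; It fetches the ball component from player pawn 0 through a GetBallRef message and checks validity before each action.
; The two movement axes apply mass-independent torque on X and Y, while Space Bar adds an upward velocity-change impulse without a ground check.
; The Start_Game input event is an empty stub.
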(event EventBeginPlay)

(event EventTick
  (params (DeltaSeconds :type Float%20%28single-precision%29)))

(event Input|AxisEvents|InputAxisMoveX_RL
  (params (AxisValue :type Float%20%28single-precision%29))
  (bind _ball (Class|IBPBPBall|GetBallRef(Message) (Game|Player|GetPlayerPawn 0)))
  (bind _ball_2 (Variables|/Game/Blueprints/BP_Ball.BP_Ball_C|GetBall _ball)
    (:then
      (Class|PrimitiveComponent|AddTorqueinRadians _ball_2 (Math|Vector|MakeVector (* AxisValue 4e+01) 0.0 0.0) "None" true))
    (:else)))

(event Input|AxisEvents|InputAxisMoveY_FB
  (params (AxisValue :type Float%20%28single-precision%29))
  (bind _ball (Class|IBPBPBall|GetBallRef(Message) (Game|Player|GetPlayerPawn 0)))
  (bind _ball_2 (Variables|/Game/Blueprints/BP_Ball.BP_Ball_C|GetBall _ball)
    (:then
      (Class|PrimitiveComponent|AddTorqueinRadians _ball_2 (Math|Vector|MakeVector 0.0 (* AxisValue 4e+01) 0.0) "None" true))
    (:else)))

(event Input|AxisEvents|InputAxisStart_Game
  (params (AxisValue :type Float%20%28single-precision%29)))

(event Input|KeyboardEvents|SpaceBar
  (params (Key :type Key%20Structure :default "None"))
  (:Pressed
    (bind _ball (Class|IBPBPBall|GetBallRef(Message) (Game|Player|GetPlayerPawn 0)))
    (bind _ball_2 (Variables|/Game/Blueprints/BP_Ball.BP_Ball_C|GetBall _ball)
      (:then
        (Physics|AddImpulse _ball_2 (Math|Vector|MakeVector 0.0 0.0 6e+02) "None" true))
      (:else))))

(fn ConstructionScript)