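; CylinderTarget is an actor Blueprint for a target that moves back and forth along a straight line.
; Each Tick offsets the actor along the normalized Direction vector by Speed scaled by delta time, without sweeping for collision.
; A looping timer started on BeginPlay reverses Direction every TimeToChange seconds.
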(event Custom|ChangeDirection
  (Variables|Default|SetDirection (* (Variables|Default|GetDirection) -1.0)))

(event EventBeginPlay
  (Utilities|Time|SetTimerbyEvent (delegate Custom|ChangeDirection) (Variables|Default|GetTimeToChange) true))

(event EventTick
  (params (DeltaSeconds :type Float%20%28single-precision%29))
  (Transformation|AddActorWorldOffset (* (Math|Vector|Normalize (Variables|Default|GetDirection)) (* (Variables|Default|GetSpeed) (Utilities|Time|GetWorldDeltaSeconds)))))

(fn ConstructionScript)